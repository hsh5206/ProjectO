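; Boss enemy Blueprint that turns to face its locked-on enemy.
; Each Tick, while that target is valid and the movement state is neither Attacking nor Death, it computes a look-at rotation and applies only the yaw.
; The rotation passes through RInterpTo with no interp speed set.
; BeginPlay, ActorBeginOverlap and the construction script are empty.
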(event EventBeginPlay)

(event Collision|EventActorBeginOverlap
  (params (OtherActor :type Actor%20Object%20Reference)))

(event EventTick
  (params (DeltaSeconds :type Float%20%28single-precision%29))
  (bind _lockedonenemy (Variables|Default|GetLockedOnEnemy))
  (bind _returnvalue (Transformation|GetActorLocation _lockedonenemy))
  (if (Math|Boolean|ANDBoolean (Utilities|IsValid (Variables|Default|GetLockedOnEnemy)) (Utilities|Enum|NotEqual(Enum) (Variables|Default|GetMovementState) "EMS_Attacking") (Utilities|Enum|NotEqual(Enum) (Variables|Default|GetMovementState) "EMS_Death"))
    (Transformation|SetActorRotation (Math|Rotator|MakeRotator 0.0 0.0 (.yaw (Math|Interpolation|RInterpTo (Transformation|GetActorRotation) (Math|Rotator|FindLookatRotation (Transformation|GetActorLocation) (Math|Vector|MakeVector (.x _returnvalue) (.y _returnvalue) (- (.z _returnvalue) 5e+01))) (Utilities|Time|GetWorldDeltaSeconds) 0.0))))))

(fn ConstructionScript)