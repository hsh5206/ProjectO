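; Player or pawn character Blueprint that handles facing and lock-on aiming every Tick.
; Outside LockOn, it smoothly yaws the actor toward its desired velocity while moving.
; In LockOn, it interpolates control rotation toward LockedOnEnemy and turns the actor to that yaw.
; The aim point sits below the target's location, with a larger drop for EnemyBoss than for Enemy.
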(event EventBeginPlay)

(event Collision|EventActorBeginOverlap
  (params (OtherActor :type Actor%20Object%20Reference)))

(event EventTick
  (params (DeltaSeconds :type Float%20%28single-precision%29))
  (bind _returnvalue (Pawn|GetController))
  (bind _lockedonenemy (Variables|Default|GetLockedOnEnemy))
  (bind _returnvalue_2 (Transformation|GetActorRotation _returnvalue))
  (bind _returnvalue_3 (Transformation|GetActorLocation _lockedonenemy))
  (Utilities|FlowControl|Sequence
    (:then_0
      (if (Utilities|Enum|NotEqual(Enum) (Variables|Default|GetCombatState) "ECS_LockOn")
        (if (Variables|Default|GetbIsMoving)
          (bind _returnvalue_4 (Class|BaseCharacter|GetDesiredVelocity self "0, 0, 0"))
          (Transformation|SetActorRotation (Math|Rotator|MakeRotator 0.0 0.0 (.yaw (Math|Interpolation|RInterpTo (Transformation|GetActorRotation) (Math|Conversions|RotationFromXVector _returnvalue_4) (Utilities|Time|GetWorldDeltaSeconds) 2.0)))))
        (else
          (Utilities|Casting|CastToEnemy _lockedonenemy
            (:then
              (Variables|Default|SetNewVar_0 5e+01))
            (:CastFailed
              (Utilities|Casting|CastToEnemyBoss _lockedonenemy)
              (Variables|Default|SetNewVar_0 1e+02)))
          (Pawn|SetControlRotation _returnvalue (Math|Rotator|MakeRotator (.Roll (Math|Rotator|BreakRotator _returnvalue_2)) (.pitch (Math|Interpolation|RInterpTo _returnvalue_2 (Math|Rotator|FindLookatRotation (Transformation|GetActorLocation) (Math|Vector|MakeVector (.x _returnvalue_3) (.y _returnvalue_3) (- (.z _returnvalue_3) (Variables|Default|GetNewVar_0)))) (Utilities|Time|GetWorldDeltaSeconds) 5.0)) (.yaw (Math|Interpolation|RInterpTo _returnvalue_2 (Math|Rotator|FindLookatRotation (Transformation|GetActorLocation) (Math|Vector|MakeVector (.x _returnvalue_3) (.y _returnvalue_3) (- (.z _returnvalue_3) (Variables|Default|GetNewVar_0)))) (Utilities|Time|GetWorldDeltaSeconds) 5.0))))
          (Transformation|SetActorRotation (Math|Rotator|MakeRotator 0.0 0.0 (.yaw (Math|Interpolation|RInterpTo (Transformation|GetActorRotation) (Math|Rotator|MakeRotator (.Roll (Math|Rotator|BreakRotator _returnvalue_2)) (.pitch (Math|Interpolation|RInterpTo _returnvalue_2 (Math|Rotator|FindLookatRotation (Transformation|GetActorLocation) (Math|Vector|MakeVector (.x _returnvalue_3) (.y _returnvalue_3) (- (.z _returnvalue_3) (Variables|Default|GetNewVar_0)))) (Utilities|Time|GetWorldDeltaSeconds) 5.0)) (.yaw (Math|Interpolation|RInterpTo _returnvalue_2 (Math|Rotator|FindLookatRotation (Transformation|GetActorLocation) (Math|Vector|MakeVector (.x _returnvalue_3) (.y _returnvalue_3) (- (.z _returnvalue_3) (Variables|Default|GetNewVar_0)))) (Utilities|Time|GetWorldDeltaSeconds) 5.0))) (Utilities|Time|GetWorldDeltaSeconds) 0.0)))))))))

(fn ConstructionScript)